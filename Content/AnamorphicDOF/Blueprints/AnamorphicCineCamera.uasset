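; Cine camera Blueprint that drives an anamorphic depth-of-field and bokeh effect.
; Construction Script and Tick run identical logic, copying lens, focus, squeeze, sampling, bokeh and depth-rejection settings into the MPC_Anamorphic_Camera parameter collection.
; Both also issue global console commands that force DOF recombine quality to zero and build a Panini distortion command, appending the value without a separating space.
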(event `self.ReceiveTick`
  (params (DeltaSeconds :type "Float (single-precision)"))
  (bind _returnvalue (`self.GetCineCameraComponent` self))
  (`KismetMaterialLibrary.SetScalarParameterValue` "/Game/AnamorphicDOF/MaterialParameterCollections/MPC_Anamorphic_Camera.MPC_Anamorphic_Camera" "FocusDistance" (`KismetMathLibrary.FClamp` (`self.AnamorphicFocusDistance`) 36.0 1000000.0))
  (`KismetMaterialLibrary.SetScalarParameterValue` "/Game/AnamorphicDOF/MaterialParameterCollections/MPC_Anamorphic_Camera.MPC_Anamorphic_Camera" "FocalLength" (`CineCameraComponent.CurrentFocalLength` _returnvalue))
  (`KismetMaterialLibrary.SetScalarParameterValue` "/Game/AnamorphicDOF/MaterialParameterCollections/MPC_Anamorphic_Camera.MPC_Anamorphic_Camera" "fStop" (`CineCameraComponent.CurrentAperture` _returnvalue))
  (`KismetMaterialLibrary.SetScalarParameterValue` "/Game/AnamorphicDOF/MaterialParameterCollections/MPC_Anamorphic_Camera.MPC_Anamorphic_Camera" "SqueezeRatio" (`self.AnamorphicSqueezeRatio`))
  (`KismetMaterialLibrary.SetScalarParameterValue` "/Game/AnamorphicDOF/MaterialParameterCollections/MPC_Anamorphic_Camera.MPC_Anamorphic_Camera" "Samples" (`self.AnamorphicSamples`))
  (`KismetMaterialLibrary.SetScalarParameterValue` "/Game/AnamorphicDOF/MaterialParameterCollections/MPC_Anamorphic_Camera.MPC_Anamorphic_Camera" "FlatBokeh" (`KismetMathLibrary.Conv_BoolToDouble` (`self.FlatBokeh`)))
  (`KismetSystemLibrary.ExecuteConsoleCommand` (`KismetStringLibrary.Concat_StrStr` (`KismetStringLibrary.Concat_StrStr` "r.upscale.Panini.D " (`KismetStringLibrary.Conv_DoubleToString` (`self.Distortion`))) " (.8)") null)
  (`KismetSystemLibrary.ExecuteConsoleCommand` "r.DOF.Recombine.Quality 0" null)
  (`KismetMaterialLibrary.SetScalarParameterValue` "/Game/AnamorphicDOF/MaterialParameterCollections/MPC_Anamorphic_Camera.MPC_Anamorphic_Camera" "EdgeRing" (`KismetMathLibrary.Conv_BoolToDouble` (`self.BokehEdgeRing`)))
  (`KismetMaterialLibrary.SetScalarParameterValue` "/Game/AnamorphicDOF/MaterialParameterCollections/MPC_Anamorphic_Camera.MPC_Anamorphic_Camera" "EdgeBias" (`self.BokehEdgeRingBias`))
  (`KismetMaterialLibrary.SetScalarParameterValue` "/Game/AnamorphicDOF/MaterialParameterCollections/MPC_Anamorphic_Camera.MPC_Anamorphic_Camera" "DepthRejection" (`KismetMathLibrary.Conv_BoolToDouble` (`self.DepthRejection`)))
  (`KismetMaterialLibrary.SetScalarParameterValue` "/Game/AnamorphicDOF/MaterialParameterCollections/MPC_Anamorphic_Camera.MPC_Anamorphic_Camera" "DepthBias" (`self.DepthRejectionBias`)))

(fn `UserConstructionScript`
  (bind _returnvalue (`self.GetCineCameraComponent` self))
  (`KismetMaterialLibrary.SetScalarParameterValue` "/Game/AnamorphicDOF/MaterialParameterCollections/MPC_Anamorphic_Camera.MPC_Anamorphic_Camera" "FocusDistance" (`KismetMathLibrary.FClamp` (`self.AnamorphicFocusDistance`) 36.0 1000000.0))
  (`KismetMaterialLibrary.SetScalarParameterValue` "/Game/AnamorphicDOF/MaterialParameterCollections/MPC_Anamorphic_Camera.MPC_Anamorphic_Camera" "FocalLength" (`CineCameraComponent.CurrentFocalLength` _returnvalue))
  (`KismetMaterialLibrary.SetScalarParameterValue` "/Game/AnamorphicDOF/MaterialParameterCollections/MPC_Anamorphic_Camera.MPC_Anamorphic_Camera" "fStop" (`CineCameraComponent.CurrentAperture` _returnvalue))
  (`KismetMaterialLibrary.SetScalarParameterValue` "/Game/AnamorphicDOF/MaterialParameterCollections/MPC_Anamorphic_Camera.MPC_Anamorphic_Camera" "SqueezeRatio" (`self.AnamorphicSqueezeRatio`))
  (`KismetMaterialLibrary.SetScalarParameterValue` "/Game/AnamorphicDOF/MaterialParameterCollections/MPC_Anamorphic_Camera.MPC_Anamorphic_Camera" "Samples" (`self.AnamorphicSamples`))
  (`KismetMaterialLibrary.SetScalarParameterValue` "/Game/AnamorphicDOF/MaterialParameterCollections/MPC_Anamorphic_Camera.MPC_Anamorphic_Camera" "FlatBokeh" (`KismetMathLibrary.Conv_BoolToDouble` (`self.FlatBokeh`)))
  (`KismetSystemLibrary.ExecuteConsoleCommand` (`KismetStringLibrary.Concat_StrStr` (`KismetStringLibrary.Concat_StrStr` "r.upscale.Panini.D " (`KismetStringLibrary.Conv_DoubleToString` (`self.Distortion`))) " (.8)") null)
  (`KismetSystemLibrary.ExecuteConsoleCommand` "r.DOF.Recombine.Quality 0" null)
  (`KismetMaterialLibrary.SetScalarParameterValue` "/Game/AnamorphicDOF/MaterialParameterCollections/MPC_Anamorphic_Camera.MPC_Anamorphic_Camera" "EdgeRing" (`KismetMathLibrary.Conv_BoolToDouble` (`self.BokehEdgeRing`)))
  (`KismetMaterialLibrary.SetScalarParameterValue` "/Game/AnamorphicDOF/MaterialParameterCollections/MPC_Anamorphic_Camera.MPC_Anamorphic_Camera" "EdgeBias" (`self.BokehEdgeRingBias`))
  (`KismetMaterialLibrary.SetScalarParameterValue` "/Game/AnamorphicDOF/MaterialParameterCollections/MPC_Anamorphic_Camera.MPC_Anamorphic_Camera" "DepthRejection" (`KismetMathLibrary.Conv_BoolToDouble` (`self.DepthRejection`)))
  (`KismetMaterialLibrary.SetScalarParameterValue` "/Game/AnamorphicDOF/MaterialParameterCollections/MPC_Anamorphic_Camera.MPC_Anamorphic_Camera" "DepthBias" (`self.DepthRejectionBias`)))