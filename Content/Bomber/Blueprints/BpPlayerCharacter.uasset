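; Player character Blueprint for the Bomber game that adds a nickname label to each character.
; On BeginPlay it creates a UI_NicknameWidget owned by the first player controller and assigns it to the character's NicknameWidgetComponent.
; The label shows the game instance's Nickname for the character with ID 0 and "AI" for all others.
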(event `self.ReceiveBeginPlay`
  (`self.CreateNickname`))

(fn `CreateNickname`
  (locals (CreatedUMGWidget :type "/Game/Bomber/UI/Nickname/UI_NicknameWidget Object Reference"))
  (bind _nickname (`/Game/Bomber/UI/Nickname/UI_NicknameWidget.Nickname` (`local.CreatedUMGWidget`)))
  (`/Engine/EditorBlueprintResources/StandardMacros.IsValid` (`self.NicknameWidgetComponent`)
    (:`Is Valid`
      (bind _returnvalue (`|CreateWidget` "/Game/Bomber/UI/Nickname/UI_NicknameWidget.UI_NicknameWidget_C" (`GameplayStatics.GetPlayerController` 0)))
      (bind _output_get (set `local.CreatedUMGWidget` _returnvalue))
      (`/Engine/EditorBlueprintResources/StandardMacros.IsValid` _output_get
        (:`Is Valid`
          (if (and (`KismetSystemLibrary.IsValid` (`SingletonLibrary.GetMyGameInstance`)) (`KismetSystemLibrary.IsValid` _nickname))
            (`TextBlock.SetText` _nickname (select `bool` (== (`self.CharacterID_`) 0) :`false` "AI" :`true` (`MyGameInstance.Nickname` (`SingletonLibrary.GetMyGameInstance`))))
            (`WidgetComponent.SetWidget` (`self.NicknameWidgetComponent`) (`local.CreatedUMGWidget`))))))))

(fn `UserConstructionScript`)