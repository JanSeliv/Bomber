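; Singleton library Blueprint whose development-only AddDebugTextRenders override draws debug labels over Bomber level cells.
; The parent function creates the text render components, then this graph sets their text, size, color and absolute transform.
; When coordinate renders exist, components pair per cell, with odd indices showing smaller X/Y coordinates offset opposite the main label.
; An empty string leaves only coordinates, and all text lies flat, aligned to the level map's rotation.
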(fn `AddDebugTextRenders`
  (params (Owner :type "Actor Object Reference") (Cells :type "Set of Cell Structure (by ref)") (TextColor :type "LinearColor Structure (by ref)") (TextHeight :type "Float (double-precision)") (TextSize :type "Float (double-precision)") (RenderString :type String) (CoordinatePosition :type "Vector Structure (by ref)"))
  (returns (bOutHasCoordinateRenders :type Boolean) (OutTextRenderComponents :type "Array of TextRenderComponent Object Reference"))
  (locals (isCoordinateRender :type Boolean) (renderComponentIt :type "TextRenderComponent Object Reference") (TextLocationIt :type "Vector Structure") (OldOwnerRenderComponents :type "Array of TextRenderComponent Object Reference") (cellLocationIt :type "Vector Structure") (RenderText :type Text))
  (bind (_celllocationit_x _celllocationit_y) (`KismetMathLibrary.BreakVector` (`local.cellLocationIt`)))
  (bind _textsize (`local.TextSize`))
  (bind _coordinateposition (`local.CoordinatePosition`))
  (bind (_celllocationit_x_2 _celllocationit_y_2 _celllocationit_z) (`KismetMathLibrary.BreakVector` (`local.cellLocationIt`)))
  (bind (_bouthascoordinaterenders _outtextrendercomponents) (`parent.AddDebugTextRenders` Owner Cells TextColor TextHeight TextSize "" CoordinatePosition)) ; Create objects of text render components
  (`|ExecutionSequence`
    (:`then_0`
      (if (> (`KismetArrayLibrary.Array_Length` _outtextrendercomponents) 0)
        ;[1 1 1] Iteration of created in the Parent text renders
        (bind _result (`BlueprintSetLibrary.Set_ToArray` (`local.Cells`)))
        (for (_array_element _array_index) _outtextrendercomponents
          (bind _output_get (set `local.renderComponentIt` _array_element))
          (`/Engine/EditorBlueprintResources/StandardMacros.IsValid` _output_get
            (:`Is Valid`
              (bind _output_location (break `Cell` (`|GetArrayItem` _result (select `bool` _bouthascoordinaterenders :`false` _array_index :`true` (`KismetMathLibrary.FFloor` (/ (`KismetMathLibrary.Conv_IntToDouble` _array_index) 2.0))))))
              (set `local.cellLocationIt` _output_location)
              (set `local.RenderText` (`KismetTextLibrary.Conv_StringToText` (`local.RenderString`)))
              (set `local.isCoordinateRender` (or (`KismetTextLibrary.TextIsEmpty` (`local.RenderText`)) (and (`KismetMathLibrary.Conv_IntToBool` (mod _array_index 2)) _bouthascoordinaterenders)))
              (`|ExecutionSequence`
                (:`then_0`
                  ;;[1 1 1] Text render location of each cell
                  (set `local.TextLocationIt` (+ (`KismetMathLibrary.MakeVector` _celllocationit_x_2 _celllocationit_y_2 (+ _celllocationit_z (`local.TextHeight`))) (select `bool` (`local.isCoordinateRender`) :`false` _coordinateposition :`true` (`KismetMathLibrary.MakeVector` (* -1 (.x _coordinateposition)) (* -1 (.y _coordinateposition)) (.z _coordinateposition))))))
                (:`then_1`
                  ;;[1 1 1] Init the text render
                  (`SceneComponent.SetAbsolute` (`local.renderComponentIt`) true true true)
                  (`TextRenderComponent.K2_SetText` (`local.renderComponentIt`) (select `bool` (`local.isCoordinateRender`) :`false` (`local.RenderText`) :`true` (`KismetTextLibrary.Conv_StringToText` (`KismetStringLibrary.Concat_StrStr` (`KismetStringLibrary.Conv_IntToString` (`KismetMathLibrary.FFloor` _celllocationit_x)) (select `bool` (>= (`local.TextSize`) 48.0) :`false` " " :`true` " \n") (`KismetStringLibrary.Conv_IntToString` (`KismetMathLibrary.FFloor` _celllocationit_y))))))
                  (`TextRenderComponent.SetWorldSize` (`local.renderComponentIt`) (select `bool` (`local.isCoordinateRender`) :`false` _textsize :`true` (/ _textsize 2.5)))
                  (`TextRenderComponent.SetHorizontalAlignment` (`local.renderComponentIt`) "EHTA_Center")
                  (`TextRenderComponent.SetVerticalAlignment` (`local.renderComponentIt`) "EVRTA_TextCenter")
                  (`TextRenderComponent.SetTextRenderColor` (`local.renderComponentIt`) (`KismetMathLibrary.Conv_LinearColorToColor` (`local.TextColor`))) ; green
                  (`SceneComponent.K2_SetWorldTransform` (`local.renderComponentIt`) (`KismetMathLibrary.MakeTransform` (`local.TextLocationIt`) (`KismetMathLibrary.ComposeRotators` (struct :`Pitch` 90.0 :`Roll` -90.0) (`Actor.K2_GetActorRotation` (`self.GetLevelMap`)))) false false))))))))
    (:`then_1`
      (return _bouthascoordinaterenders _outtextrendercomponents))))