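; Base actor for a rotating showcase of level meshes on stacked floors, which becomes the player's view target.
; Construction script builds a floor per data asset of ActorType, ringing it with static or skeletal meshes while preserving per-mesh transform tweaks by name.
; Timelines raise the floor stack or rotate the current floor to change selection, then hide the previous mesh.
; The selected mesh spins on Tick; static ones support an inverted-material outline.
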(event `self.ReceiveBeginPlay`
  (`parent.ReceiveBeginPlay`)
  (`|ExecutionSequence`
    (:`then_0`
      (`self.UpdateCurrentFloorComp`)
      (`self.SetCurrentMeshComp` (`self.GetFirstMeshIndOfCurFloor`)))
    (:`then_1`
      (`KismetSystemLibrary.Delay` 0.2)
      (`PlayerController.SetViewTargetWithBlend` (`GameplayStatics.GetPlayerController` 0) self 0.0 "VTBlend_Linear" 0.0 false))))

(event `self.ReceiveTick`
  (params (DeltaSeconds :type "Float (single-precision)"))
  (`|ExecutionSequence`
    (:`then_0`
      (bind _currentmeshcomp (`self.CurrentMeshComp`)
        (:`then`
          (`SceneComponent.K2_AddRelativeRotation` _currentmeshcomp (`KismetMathLibrary.MakeRotator` 0.0 0.0 (`|GetArrayItem` (`self.MeshRotationSpeeds`))) false false))
        (:`else`)))))

(event `RaiseFloor_Internal`
  (bind (_initialfloorlocation_x _initialfloorlocation_y _initialfloorlocation_z) (`KismetMathLibrary.BreakVector` (`self.InitialFloorLocation`)))
  ;[1 1 1] Internal functions. Are not for direct using!
  (`self.FloorsRoot`
    (:`then`
      (if (not (`self.InFloorRaising`))
        (set `self.InFloorRaising` true)
        (bind (_direction _newtrack_0) (`Timeline|Timeline_1` :!via `PlayFromStart`)
          (:`Update`
            (`SceneComponent.K2_SetRelativeLocation` (`self.FloorsRoot`) (`KismetMathLibrary.MakeVector` _initialfloorlocation_x _initialfloorlocation_y (`self.InterpTo` _initialfloorlocation_z _newtrack_0 (`self.TargetFloorHeight`))) false false))
          (:`Finished`
            (set `self.InFloorRaising` false)
            (`self.HideLastMesh`)
            (`self.UpdateCurrentFloorComp`)))))
    (:`else`)))

(event `RotateFloor_Internal`
  (bind (_initialfloorrotation_roll _initialfloorrotation_pitch _initialfloorrotation_yaw) (`KismetMathLibrary.BreakRotator` (`self.InitialFloorRotation`)))
  ;[1 1 1] Internal functions. Are not for direct using!
  (`self.CurrentFloorComp`
    (:`then`
      (if (not (`self.InFloorRotating`))
        (set `self.InFloorRotating` true)
        (bind (_direction _newtrack_0) (`Timeline|Timeline_0` :!via `PlayFromStart`)
          (:`Update`
            (`SceneComponent.K2_SetRelativeRotation` (`self.CurrentFloorComp`) (`KismetMathLibrary.MakeRotator` _initialfloorrotation_roll _initialfloorrotation_pitch (`self.InterpTo` _initialfloorrotation_yaw _newtrack_0 (`self.TargetFloorAngle`))) false true))
          (:`Finished`
            (set `self.InFloorRotating` false)
            (`self.HideLastMesh`)))))
    (:`else`)))

(event `Up`
  ;[1 1 1] Debug
  (`self.RaiseFloor` -1))

(event `Down`
  ;[1 1 1] Debug
  (`self.RaiseFloor` 1))

(event `Left`
  ;[1 1 1] Debug
  (`self.RotateFloor` -1))

(event `Right`
  ;[1 1 1] Debug
  (`self.RotateFloor` 1))

(fn `GetFirstMeshIndOfCurFloor`
  (returns (MeshNo :type Integer))
  (locals (LenCount :type Integer :default -1))
  (`|ExecutionSequence`
    (:`then_0`
      (for (_array_element _array_index) (`self.Floors`)
        (if (== (`self.CurrentFloorInd`) _array_index)
          (`/Engine/EditorBlueprintResources/StandardMacros.IncrementInt` (`local.LenCount`)
            (:`  `
              (break)))
          (else
            (set `local.LenCount` (+ (`BlueprintMapLibrary.Map_Length` (break `/Game/Bomber/Blueprints/Render/FFloor` _array_element)) (`local.LenCount`)))))))
    (:`then_1`
      (return (`local.LenCount`)))))

(fn `GetMeshRow`
  (params (FloorIndex :type Integer) (MeshIndex :type Integer))
  (returns (MeshRow :type "LevelActorMeshRow Structure (by ref)"))
  (locals (FoundIndex :type Integer :default 0) (FoundTranform :type "Transform Structure"))
  (`|ExecutionSequence`
    (:`then_0`
      (for (_array_element _array_index) (`self.Floors`)
        (bind _returnvalue (== _array_index (`local.FloorIndex`)))
        (set `local.FoundIndex` (+ (`local.FoundIndex`) (select `bool` _returnvalue :`false` (`BlueprintMapLibrary.Map_Length` (break `/Game/Bomber/Blueprints/Render/FFloor` _array_element)) :`true` (`local.MeshIndex`))))
        (if _returnvalue
          (break))))
    (:`then_1`
      (return (select `bool` (`KismetArrayLibrary.Array_IsValidIndex` (`self.RowsInternal`) (`local.FoundIndex`)) :`true` (`|GetArrayItem` (`self.RowsInternal`) (`local.FoundIndex`)))))))

(fn `HideLastMesh`
  (bind _lastmeshcomp (`self.LastMeshComp`)
    (:`then`
      (`SceneComponent.SetHiddenInGame` _lastmeshcomp true false))
    (:`else`)))

(fn `RaiseFloor`
  (params (IncrementedVal :type Integer :default 1))
  (returns (bIsLastFloor :type Boolean))
  (locals (NewFloorInd :type Integer :default -1) (FoundFloorComp :type "SceneComponent Object Reference"))
  (bind _newfloorind (`local.NewFloorInd`))
  (if (`KismetMathLibrary.BooleanNOR` (== IncrementedVal 0) (`self.InFloorRaising`))
    (`|ExecutionSequence`
      (:`then_0`
        (if (`KismetMathLibrary.BooleanNOR` (== (`local.IncrementedVal`) 0) (`self.InFloorRaising`))
          (set `local.NewFloorInd` (+ (`local.IncrementedVal`) (`self.CurrentFloorInd`)))
          (if (`KismetArrayLibrary.Array_IsValidIndex` (`self.FloorComponents`) (`local.NewFloorInd`))
            (set `self.CurrentFloorInd` (`local.NewFloorInd`))
            (bind _output_get (set `local.FoundFloorComp` (`|GetArrayItem` (`self.FloorComponents`) (`self.CurrentFloorInd`))))
            (`/Engine/EditorBlueprintResources/StandardMacros.IsValid` _output_get
              (:`Is Valid`
                (`|ExecutionSequence`
                  (:`then_0`
                    (set `self.TargetFloorHeight` (* (`local.IncrementedVal`) (`self.FloorHeight`)))
                    (set `self.InitialFloorLocation` (`SceneComponent.RelativeLocation` (`self.FloorsRoot`))))
                  (:`then_1`
                    (`self.SetCurrentMeshComp` (`self.GetFirstMeshIndOfCurFloor`))
                    (`self.RaiseFloor_Internal`))))))))
      (:`then_1`
        (return (or (== (`KismetArrayLibrary.Array_LastIndex` (`self.FloorComponents`)) _newfloorind) (== _newfloorind 0)))))))

(fn `RotateFloor`
  (params (IncrementedVal :type Integer :default 1))
  (locals (RelativeMeshInd :type Integer :default 0) (FloorMeshesN :type Integer :default 0) (FirstMeshIndOnFloor :type Integer :default 0) (NewCurrentMeshInd :type Integer :default 0))
  (bind _relativemeshind (`local.RelativeMeshInd`))
  (bind _relativemeshind_2 (`local.RelativeMeshInd`))
  (bind _returnvalue (+ (`local.FirstMeshIndOnFloor`) (`local.FloorMeshesN`)))
  (bind _output_meshes (break `/Game/Bomber/Blueprints/Render/FFloor` (`|GetArrayItem` (`self.Floors`) (`self.CurrentFloorInd`))))
  (if (`KismetMathLibrary.BooleanNOR` (== IncrementedVal 0) (`self.InFloorRotating`))
    (`|ExecutionSequence`
      (:`then_0`
        (if (`KismetArrayLibrary.Array_IsValidIndex` (`self.Floors`) (`self.CurrentFloorInd`))
          (bind _output_get (set `local.FloorMeshesN` (`BlueprintMapLibrary.Map_Length` _output_meshes)))
          (bind _returnvalue_2 (/ 360.0 (`KismetMathLibrary.Conv_IntToDouble` _output_get)))
          (set `self.TargetFloorAngle` (select `bool` (> (`local.IncrementedVal`) 0) :`false` _returnvalue_2 :`true` (* -1 _returnvalue_2)))
          (else
            (return))))
      (:`then_1`
        (set `local.FirstMeshIndOnFloor` (`self.GetFirstMeshIndOfCurFloor`))
        (bind _output_get_2 (set `local.NewCurrentMeshInd` (+ (`self.CurrentMeshInd`) (`local.IncrementedVal`))))
        (set `local.RelativeMeshInd` (- _output_get_2 (`local.FirstMeshIndOnFloor`)))
        (`self.SetCurrentMeshComp` (select `bool` (< _relativemeshind 0) :`false` (select `bool` (>= _relativemeshind_2 (`local.FloorMeshesN`)) :`false` (`local.NewCurrentMeshInd`) :`true` (- _returnvalue _relativemeshind_2)) :`true` (+ _returnvalue _relativemeshind))))
      (:`then_2`
        (set `self.InitialFloorRotation` (`SceneComponent.RelativeRotation` (`self.CurrentFloorComp`)))
        (`self.RotateFloor_Internal`)))))

(fn `SetCurrentMeshComp`
  (params (NewCurrentMeshNo :type Integer))
  (locals (FoundMesh :type "MeshComponent Object Reference"))
  (if (`KismetArrayLibrary.Array_IsValidIndex` (`self.MeshComponents`) (`local.NewCurrentMeshNo`))
    (bind _output_get (set `local.FoundMesh` (`|GetArrayItem` (`self.MeshComponents`) (`local.NewCurrentMeshNo`))))
    (`/Engine/EditorBlueprintResources/StandardMacros.IsValid` _output_get
      (:`Is Valid`
        (`|ExecutionSequence`
          (:`then_0`
            (bind _currentmeshcomp (`self.CurrentMeshComp`)
              (:`then`
                (`SceneComponent.K2_SetRelativeRotation` _currentmeshcomp (`self.InitialMeshRotation`) false true) ; reset rotation for last mesh
              )
              (:`else`)))
          (:`then_1`
            (`SceneComponent.SetHiddenInGame` (`local.FoundMesh`) false false))
          (:`then_2`
            (set `self.CurrentMeshInd` (`local.NewCurrentMeshNo`))
            (set `self.InitialMeshRotation` (`SceneComponent.RelativeRotation` (`local.FoundMesh`)))
            (set `self.LastMeshComp` (`self.CurrentMeshComp`))
            (set `self.CurrentMeshComp` (`local.FoundMesh`))))))))

(fn `SetOutline`
  (params (bShouldEnable :type Boolean))
  (bind _currentmeshcomp (`self.CurrentMeshComp`)
    (:`then`
      (if bShouldEnable
        (bind _asstatic_mesh_component (cast `StaticMeshComponent` _currentmeshcomp))
        (bind _returnvalue (`AddComponent|NODE_AddStaticMeshComponent-3` :`RelativeTransform` (`SceneComponent.GetRelativeTransform` _asstatic_mesh_component)))
        (bind _returnvalue_2 (`StaticMeshComponent.SetStaticMesh` _returnvalue (`StaticMeshComponent.StaticMesh` _asstatic_mesh_component)))
        (if _returnvalue_2
          (`PrimitiveComponent.SetMaterial` _returnvalue 0 "/Game/Bomber/Materials/Render/MI_Inverted.MI_Inverted")
          (`SceneComponent.K2_AttachToComponent` _returnvalue _asstatic_mesh_component "None" "SnapToTarget" "SnapToTarget" "SnapToTarget" true)
          (else
            (`ActorComponent.K2_DestroyComponent` _returnvalue)))
        (else
          (bind _asstatic_mesh_component_2 (cast `StaticMeshComponent` (`SceneComponent.GetChildComponent` _currentmeshcomp 0)))
          (`ActorComponent.K2_DestroyComponent` _asstatic_mesh_component_2))))
    (:`else`)))

(fn `SwitchMeshRotationSpeed`
  (`KismetArrayLibrary.Array_Swap` (`self.MeshRotationSpeeds`) 0 1))

(fn `UpdateCurrentFloorComp`
  (locals (FoundFloorComp :type "SceneComponent Object Reference"))
  (if (`KismetArrayLibrary.Array_IsValidIndex` (`self.FloorComponents`) (`self.CurrentFloorInd`))
    (`|ExecutionSequence`
      (:`then_0`
        (bind _currentfloorcomp (`self.CurrentFloorComp`)
          (:`then`
            (`SceneComponent.K2_SetRelativeRotation` :`self` _currentfloorcomp) ; reset rotation of last floor
          )
          (:`else`)))
      (:`then_1`
        (bind _output_get (set `local.FoundFloorComp` (`|GetArrayItem` (`self.FloorComponents`) (`self.CurrentFloorInd`))))
        (`/Engine/EditorBlueprintResources/StandardMacros.IsValid` _output_get
          (:`Is Valid`
            (set `self.CurrentFloorComp` (`local.FoundFloorComp`))))))))

(fn `UserConstructionScript`
  (locals (It :type "/Game/Bomber/Blueprints/Render/FFloor Structure") (CurrentHeight :type "Float (double-precision)") (AddedFloorComp :type "StaticMeshComponent Object Reference") (R :type "Float (double-precision)" :default 0.0) (CurentAngle :type "Float (double-precision)" :default 0.0) (AddedComponent :type "SceneComponent Object Reference") (CurrentLocation :type "Vector Structure" :default (0.0 0.0 0.0)) (FoundRowsOnFloor :type "Array of LevelActorMeshRow Structure") (FoundDataAssets :type "Array of LevelActorDataAsset Object Reference") (CopiedFloors :type "Array of /Game/Bomber/Blueprints/Render/FFloor Structure") (MeshIndex :type Integer) (MeshesAngle :type "Float (double-precision)") (FoundTransform :type "Transform Structure" :default "0.000000,0.000000,100.000000|0.000000,0.000000,0.000000|1.000000,1.000000,1.000000") (FloorToAdd :type "/Game/Bomber/Blueprints/Render/FFloor Structure"))
  (bind _r (`local.R`))
  (bind _curentangle (`local.CurentAngle`))
  (bind _it_meshes (break `/Game/Bomber/Blueprints/Render/FFloor` (`local.It`)))
  (bind _floortoadd_meshes (break `/Game/Bomber/Blueprints/Render/FFloor` (`local.FloorToAdd`)))
  (bind _it_meshes_2 (break `/Game/Bomber/Blueprints/Render/FFloor` (`local.It`)))
  (`|ExecutionSequence`
    (:`then_0`
      (bind _arrayindex (`/Engine/EditorBlueprintResources/StandardMacros.ReverseForEachLoop` (`self.Floors`))
        (:`LoopBody`
          (bind _output_meshes (break `/Game/Bomber/Blueprints/Render/FFloor` (`|GetArrayItem` (`self.Floors`) _arrayindex)))
          (`BlueprintMapLibrary.Map_Remove` _output_meshes))))
    (:`then_1`
      (set `local.CopiedFloors` (`self.Floors`))
      (`KismetArrayLibrary.Array_Clear` (`self.Floors`))
      (`KismetArrayLibrary.Array_Clear` (`self.RowsInternal`))
      (`KismetArrayLibrary.Array_Clear` (`self.FloorComponents`))
      (`KismetArrayLibrary.Array_Clear` (`self.MeshComponents`)))
    (:`then_2`
      (bind _output_get (set `local.FoundDataAssets` (`SingletonLibrary.GetDataAssetsByActorTypes` (`self.ActorType`))))
      (for _array_element _output_get
        (`/Engine/EditorBlueprintResources/StandardMacros.IsValid` _array_element
          (:`Is Valid`
            (`|ExecutionSequence`
              (:`then_0`
                (set `local.FoundRowsOnFloor` (`LevelActorDataAsset.GetMeshesByLevelType` _array_element 7))
                (set `local.FloorToAdd` (struct)))
              (:`then_1`
                (for _array_element_2 (`local.FoundRowsOnFloor`)
                  (`KismetArrayLibrary.Array_Add` (`self.RowsInternal`) _array_element_2)
                  (bind _returnvalue (`KismetSystemLibrary.GetDisplayName` (`.Mesh` (break `LevelActorMeshRow` _array_element_2))))
                  (if (not (`KismetStringLibrary.IsEmpty` _returnvalue))
                    (`|ExecutionSequence`
                      (:`then_0`
                        (for _array_element_3 (`local.CopiedFloors`)
                          (bind (_value _returnvalue_2) (`BlueprintMapLibrary.Map_Find` (break `/Game/Bomber/Blueprints/Render/FFloor` _array_element_3) _returnvalue))
                          (if _returnvalue_2
                            (set `local.FoundTransform` _value)
                            (break))))
                      (:`then_1`
                        (`BlueprintMapLibrary.Map_Add` _floortoadd_meshes _returnvalue (`local.FoundTransform`)))))))
              (:`then_2`
                (`KismetArrayLibrary.Array_Add` (`self.Floors`) (`local.FloorToAdd`))))))))
    (:`then_3`
      (for (_array_element_4 _array_index) (`self.Floors`)
        (`|ExecutionSequence`
          (:`then_0`
            (set `local.It` _array_element_4)
            (bind _returnvalue_3 (`AddComponent|NODE_AddStaticMeshComponent-0` :`RelativeTransform` (`KismetMathLibrary.MakeTransform` (`KismetMathLibrary.MakeVector` 0.0 0.0 (`local.CurrentHeight`)) (struct) (30.0 30.0 0.1))))
            (bind _output_get_2 (set `local.AddedFloorComp` _returnvalue_3))
            (`KismetArrayLibrary.Array_Add` (`self.FloorComponents`) _output_get_2)
            (set `local.R` (`.SphereRadius` (`KismetSystemLibrary.GetComponentBounds` (`local.AddedFloorComp`))))
            (`SceneComponent.K2_AttachToComponent` (`local.AddedFloorComp`) (`self.FloorsRoot`) "None" "KeepWorld" "KeepWorld" "KeepWorld" true))
          (:`then_1`
            (set `local.MeshesAngle` (/ 360.0 (`KismetMathLibrary.Conv_IntToDouble` (`BlueprintMapLibrary.Map_Length` _it_meshes))))
            (bind _values (`BlueprintMapLibrary.Map_Values` _it_meshes_2))
            (for (_array_element_5 _array_index_2) _values
              (set `local.MeshIndex` _array_index_2)
              (set `local.CurrentLocation` (`KismetMathLibrary.MakeVector` (* (`KismetMathLibrary.DegCos` _curentangle) _r) (* _r (`KismetMathLibrary.DegSin` _curentangle)) (`local.CurrentHeight`)))
              (`|ExecutionSequence`
                (:`then_0`
                  (if (== 0 (`local.MeshIndex`))
                    (bind _returnvalue_4 (`AddComponent|NODE_AddBillboardComponent-0` :`RelativeTransform` (`KismetMathLibrary.MakeTransform` (`local.CurrentLocation`) (struct) (2.5 2.5 2.5))))
                    (set `local.AddedComponent` _returnvalue_4)
                    (set `SceneComponent.bAbsoluteScale` true (`local.AddedComponent`))
                    (`SceneComponent.K2_AttachToComponent` (`local.AddedComponent`) (`local.AddedFloorComp`) "None" "KeepWorld" "KeepWorld" "KeepWorld" true :!label _label)))
                (:`then_1`
                  (bind (_meshrow_leveltype _meshrow_mesh) (break `LevelActorMeshRow` (`self.GetMeshRow` _array_index (`local.MeshIndex`))))
                  (bind _asstatic_mesh (cast `StaticMesh` _meshrow_mesh))
                  (bind _rotation (.rotation _array_element_5))
                  (bind _scale (.scale _array_element_5))
                  (bind _returnvalue_5 (+ (`local.CurrentLocation`) (.location _array_element_5)))
                  (bind _returnvalue_6 (`AddComponent|NODE_AddStaticMeshComponent-1` :`RelativeTransform` (`KismetMathLibrary.MakeTransform` _returnvalue_5 _rotation _scale)))
                  (`StaticMeshComponent.SetStaticMesh` _returnvalue_6 _asstatic_mesh)
                  (set `local.AddedComponent` _returnvalue_6)
                  (bind _asmesh_component (cast `MeshComponent` (`local.AddedComponent`) :!label _label_2))
                  (`KismetArrayLibrary.Array_Add` (`self.MeshComponents`) _asmesh_component)
                  (set `local.CurentAngle` (+ (`local.CurentAngle`) (`local.MeshesAngle`)))
                  (goto _label))
                (:`then_2`
                  (bind _asskeletal_mesh (cast `SkeletalMesh` _meshrow_mesh))
                  (bind _returnvalue_7 (`AddComponent|NODE_AddSkeletalMeshComponent-0` :`RelativeTransform` (`KismetMathLibrary.MakeTransform` _returnvalue_5 _rotation _scale)))
                  (`SkinnedMeshComponent.SetSkinnedAssetAndUpdate` _returnvalue_7 _asskeletal_mesh true)
                  (set `local.AddedComponent` _returnvalue_7)
                  (goto _label_2)))))
          (:`then_2`
            (set `local.CurrentHeight` (- (`local.CurrentHeight`) (`self.FloorHeight`)))))))))