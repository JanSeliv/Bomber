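; BP_PlayerCharacter is the Blueprint for a Bomber player character that sets up the nickname widget shown on the character.
; UpdateNickname fetches a WBP_Nickname from the HUD by the internal character ID and assigns it to the nickname widget component.
; The character with ID zero gets the nickname from the game instance, while all others are labeled "AI".
; BeginPlay and the construction script only call their parent versions.
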(event `self.ReceiveBeginPlay`
  (`parent.ReceiveBeginPlay`))

(fn `UpdateNickname`
  (locals (NicknameWidget :type "/Game/Bomber/UI/Nickname/WBP_Nickname Object Reference"))
  (bind _returnvalue (`SingletonLibrary.GetMyHUD`))
  (bind _returnvalue_2 (`SingletonLibrary.GetMyGameInstance`))
  (bind _characteridinternal (`self.CharacterIDInternal`))
  (`parent.UpdateNickname`)
  (`self.NicknameWidgetComponent`
    (:`then`
      (`/Engine/EditorBlueprintResources/StandardMacros.IsValid` _returnvalue
        (:`Is Valid`
          (bind _aswbp_nickname (cast `/Game/Bomber/UI/Nickname/WBP_Nickname` (`MyHUD.GetNicknameWidget` _returnvalue (`self.CharacterIDInternal`))))
          (set `local.NicknameWidget` _aswbp_nickname)
          (`/Engine/EditorBlueprintResources/StandardMacros.IsValid` _returnvalue_2
            (:`Is Valid`
              (`/Game/Bomber/UI/Nickname/WBP_Nickname.SetNickname` (`local.NicknameWidget`) (select `bool` (== _characteridinternal 0) :`false` "AI" :`true` (`MyGameInstance.Nickname` _returnvalue_2)) _characteridinternal)
              (`WidgetComponent.SetWidget` (`self.NicknameWidgetComponent`) (`local.NicknameWidget`)))))))
    (:`else`)))

(fn `UserConstructionScript`
  (`parent.UserConstructionScript`))