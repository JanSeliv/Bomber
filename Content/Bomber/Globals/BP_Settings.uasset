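; BP_Settings is a settings Blueprint for the Bomber game that builds its setting controls from a Data Table.
; InitSettings defers to the parent, which calls the Add functions from that table.
; The Add overrides cover buttons, button rows, checkboxes, comboboxes, sliders, text inputs and simple text.
; Each override only forwards its data to the parent implementation, so this Blueprint adds no logic of its own.
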(fn `AddSettingsButton`
  (params (Data :type "SettingsButton Structure (by ref)"))
  (`parent.AddSettingsButton` Data))

(fn `AddSettingsButtonsRow`
  (params (Data :type "SettingsButtonsRow Structure (by ref)"))
  (`parent.AddSettingsButtonsRow` Data))

(fn `AddSettingsCheckbox`
  (params (Data :type "SettingsCheckbox Structure (by ref)"))
  (`parent.AddSettingsCheckbox` Data))

(fn `AddSettingsCombobox`
  (params (Data :type "SettingsCombobox Structure (by ref)"))
  (`parent.AddSettingsCombobox` Data))

(fn `AddSettingsSlider`
  (params (Data :type "SettingsSlider Structure (by ref)"))
  (`parent.AddSettingsSlider` Data))

(fn `AddSettingsTextInput`
  (params (Data :type "SettingsTextInput Structure (by ref)"))
  (`parent.AddSettingsTextInput` Data))

(fn `AddSettingsTextSimple`
  (params (Data :type "SettingsTextSimple Structure (by ref)"))
  (`parent.AddSettingsTextSimple` Data))

(fn `InitSettings`
  (`|ExecutionSequence`
    (:`then_1`
      (`parent.InitSettings`) ; Calls Add functions by Data Table
      (return))))